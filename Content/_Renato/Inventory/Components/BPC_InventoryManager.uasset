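; Player inventory component that manages typed sword, shield and item slots, money, health and their UI widgets.
; A per-tick forward sphere trace shows the interact popup; the pickup input adds items using DT_Items stack sizes.
; Only general items split overflow into empty slots or respawn it on the floor, while upgrade packs enlarge slot arrays.
; Capsule overlap collects money, the toggle input opens a paused inventory, and N/M keys test healing and damage.
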(event EventBeginPlay
  (bind _playerinventory (Variables|Default|GetPlayerInventory))
  (bind (_sword _shields _items) (Utilities|Struct|BreakS_ItemsManager _playerinventory))
  ;[0 0.5733 1] Mapping, and obtaining important information
  (Input|AddMappingContext (PlayerController|LocalPlayerSubsystems|GetEnhancedInputLocalPlayerSubsystem (Game|GetPlayerController 0)) "/Game/_Renato/Inventory/Inputs/IMC_InventoryInputs.IMC_InventoryInputs" 0 "(bIgnoreAllPressedKeysUntilRelease=True,bForceImmediately=False)")
  (bind _returnvalue (UserInterface|CreateWidget "/Game/_Renato/Inventory/Widgets/WBP_Inventory.WBP_Inventory_C"))
  (Variables|Widgets|SetWBP_InventoryWidget _returnvalue)
  (bind _asbp_third_person_character (Utilities|Casting|CastToBP_ThirdPersonCharacter (Game|GetPlayerCharacter 0)))
  (bind _output_get (Variables|Scripts|SetBP%20Third%20Person%20Character _asbp_third_person_character))
  ;[0 0.5997 1] Bind to event
  (Collision|BindEventtoOnComponentBeginOverlap (Variables|/Script/Engine.Character|GetCapsuleComponent _output_get) (EventDispatchers|CreateEvent :!event MoneyPickUp))
  ;[0 0.4984 1] Initialize interaction widget
  (bind _returnvalue_2 (UserInterface|CreateWidget "/Game/_Renato/Inventory/Widgets/WBP_Interact.WBP_Interact_C"))
  (Variables|Widgets|SetWBP_Interact _returnvalue_2)
  ;[0 0.7223 1] Initialize inventory slot size
  (Utilities|Array|Resize _sword 1)
  (Utilities|Array|Resize _shields 3)
  (Utilities|Array|Resize _items 4)
  ;[0 0.3769 1] Update Items in inventory in UI
  (Default|UpdateItemsinInventoryUI (Variables|Widgets|GetWBP_InventoryWidget) (Variables|Default|GetPlayerInventory)))

(event EventTick
  (params (DeltaSeconds :type Float%20%28single-precision%29))
  (bind _wbp_interact (Variables|Widgets|GetWBP_Interact))
  ;[0 0.4549 1] Popus
  (bind (_item _founditem) (Items|TraceItemtoPickUp))
  (Variables|/Game/_Renato/Inventory/Widgets/WBP_InfoPopup.WBP_InfoPopup_C|SetItem (Variables|/Game/_Renato/Inventory/Widgets/WBP_Interact.WBP_Interact_C|GetWBP_InfoPopup (Variables|Widgets|GetWBP_Interact)) _item)
  (if _founditem
    (UserInterface|Viewport|AddtoViewport _wbp_interact 0)
    (else
      (Widget|RemovefromParent _wbp_interact))))

(event Input|KeyboardEvents|N
  (params (Key :type Key%20Structure))
  (:Pressed
    (Health|IncreaseHealth 0.5)))

(event Input|KeyboardEvents|M
  (params (Key :type Key%20Structure))
  (:Pressed
    (Health|DealDamage 0.5)))

(event Input|EnhancedActionEvents|EnhancedInputActionIA_Pickup
  (params (ActionValue :type Boolean) (ElapsedSeconds :type Float%20%28double-precision%29) (TriggeredSeconds :type Float%20%28double-precision%29) (InputAction :type Input%20Action%20Object%20Reference :default "/Game/_Renato/Inventory/Inputs/IA_Pickup.IA_Pickup"))
  ;[0.06801 0.6096 1] Add to inventory
  (:Triggered
    (bind (_item _founditem _itemactor) (Items|TraceItemtoPickUp))
    (if _founditem
      (bind _success (Items|AddtoInventory _item _itemactor))
      (if _success
        (Actor|DestroyActor _itemactor)
        ;[0 0.3769 1] Update Items in inventory in UI
        (Default|UpdateItemsinInventoryUI (Variables|Widgets|GetWBP_InventoryWidget) (Variables|Default|GetPlayerInventory))
        (else
          (Development|PrintString "Full inventory"))))))

(event Input|EnhancedActionEvents|EnhancedInputActionIA_InventoryToggle
  (params (ActionValue :type Boolean) (ElapsedSeconds :type Float%20%28double-precision%29) (TriggeredSeconds :type Float%20%28double-precision%29) (InputAction :type Input%20Action%20Object%20Reference :default "/Game/_Renato/Inventory/Inputs/IA_InventoryToggle.IA_InventoryToggle"))
  (bind _returnvalue (Game|GetPlayerController 0))
  (bind _wbp_inventorywidget (Variables|Widgets|GetWBP_InventoryWidget))
  ;[0 0.6211 1] Open Inventory
  (:Triggered
    (UserInterface|Viewport|AddtoViewport (Variables|Widgets|GetWBP_InventoryWidget) 0)
    (Variables|/Script/Engine.PlayerController|SetbShowMouseCursor _returnvalue true)
    (Input|SetInputModeUIOnly _returnvalue _wbp_inventorywidget "DoNotLock" false)
    (Game|SetGamePaused true)
    (Default|UpdateItemsinInventoryUI _wbp_inventorywidget (Variables|Default|GetPlayerInventory))))

(fn MoneyPickUp
  (params (OverlappedComponent :type Primitive%20Component%20Object%20Reference) (OtherActor :type Actor%20Object%20Reference) (OtherComp :type Primitive%20Component%20Object%20Reference) (OtherBodyIndex :type Integer) (bFromSweep :type Boolean) (SweepResult :type Hit%20Result%20Structure%20%28by%20ref%29))
  ;[0 0.5181 1] Pickup money
  (bind _asbp_money (Utilities|Casting|CastToBP_Money OtherActor))
  (bind _returnvalue (Utilities|GetDataTableRow "/Game/_Renato/Inventory/Data_Tables/Money_DT/DT_Money.DT_Money" (.rowname (Variables|/Game/_Renato/Inventory/Blueprints/MoneySystem/BP_Money.BP_Money_C|GetMoneyType _asbp_money)))
    (:then
      (bind _output_get (Variables|Money|SetMoneyAmountComponent (+ (Variables|Money|GetMoneyAmountComponent) (.amount _returnvalue))))
      (Actor|DestroyActor _asbp_money)
      (Variables|/Game/_Renato/Inventory/Widgets/WBP_Inventory.WBP_Inventory_C|SetMoneyAmountInventory (Variables|Widgets|GetWBP_InventoryWidget) _output_get) ; Update UI money when picked up
      (return))))

(fn IncreaseHealth
  (params (HealthRestored :type Float%20%28double-precision%29))
  (bind _maxhealth (Variables|Health|GetMaxHealth))
  (if (== (Variables|Health|GetCurrentHealth) _maxhealth)
    (return false)
    (else
      (if (>= HealthRestored (- _maxhealth (Variables|Health|GetCurrentHealth)))
        (Variables|Health|SetCurrentHealth (Variables|Health|GetMaxHealth))
        (else
          (Variables|Health|SetCurrentHealth (+ HealthRestored (Variables|Health|GetCurrentHealth)))))
      (Default|UpdateHealthBar (Variables|Widgets|GetWBP_HealthBar))
      (Default|UpdateHealthBar (Variables|/Game/_Renato/Inventory/Widgets/WBP_Inventory.WBP_Inventory_C|GetWBP_HealthBar (Variables|Widgets|GetWBP_InventoryWidget)))
      (return true))))

(fn DealDamage
  (params (Damage :type Float%20%28double-precision%29))
  (Variables|Health|SetCurrentHealth (- (Variables|Health|GetCurrentHealth) Damage))
  ;[0 0.5238 1] Update hud health bar
  (Default|UpdateHealthBar (Variables|Widgets|GetWBP_HealthBar))
  ;[0 0.5946 1] Update inventory health bar
  (Default|UpdateHealthBar (Variables|/Game/_Renato/Inventory/Widgets/WBP_Inventory.WBP_Inventory_C|GetWBP_HealthBar (Variables|Widgets|GetWBP_InventoryWidget))))

(fn GenerateHealthBar
  (bind _returnvalue (UserInterface|CreateWidget "/Game/_Renato/Inventory/Widgets/WBP_HealthBar.WBP_HealthBar_C"))
  (bind _output_get (Variables|Widgets|SetWBP_HealthBar _returnvalue))
  (Class|UserWidget|SetPositioninViewport _output_get "(X=10.000000,Y=10.000000)" true)
  (UserInterface|Viewport|AddtoViewport _output_get 0))

(fn TraceItemtoPickUp
  (bind _returnvalue (Game|GetPlayerCharacter 0))
  (bind _returnvalue_2 (Transformation|GetActorLocation _returnvalue))
  (bind _returnvalue_3 (- _returnvalue_2 "0.000000,0.000000,60.000000"))
  (bind _outhit (Collision|SphereTraceByChannel _returnvalue_3 (+ (* (Transformation|GetActorForwardVector _returnvalue) 8e+01) _returnvalue_3) 3e+01 "TraceTypeQuery1" false 0 "ForOneFrame"))
  (bind _asbp_items (Utilities|Casting|CastToBP_Items (.hitactor _outhit))
    (:then
      (return (Variables|/Game/_Renato/Inventory/Blueprints/Items/BP_Items.BP_Items_C|GetItem _asbp_items) true (.hitactor _outhit)))
    (:CastFailed
      (return "" false 0))))

(fn AddtoInventory
  (params (Item :type S%20Slots%20Structure) (ItemActor :type Actor%20Object%20Reference))
  (bind (_itemid _quantity _itemtype) (Utilities|Struct|BreakS_Slots Item))
  (bind (_itemid_2 _quantity_2 _itemtype_2) (Utilities|Struct|BreakS_Slots Item))
  (bind _quantity_3 (Utilities|Struct|BreakS_Slots Item))
  (bind (_itemid_3 _quantity_4 _itemtype_3) (Utilities|Struct|BreakS_Slots Item))
  (bind (_itemid_4 _quantity_5 _itemtype_4) (Utilities|Struct|BreakS_Slots Item))
  (bind (_itemid_5 _quantity_6) (Utilities|Struct|BreakS_Slots Item))
  (bind (_itemid_6 _quantity_7 _itemtype_5) (Utilities|Struct|BreakS_Slots Item))
  (bind (_itemid_7 _quantity_8 _itemtype_6) (Utilities|Struct|BreakS_Slots Item))
  (bind (_itemid_8 _quantity_9 _itemtype_7) (Utilities|Struct|BreakS_Slots Item))
  (bind (_itemid_9 _quantity_10 _itemtype_8) (Utilities|Struct|BreakS_Slots Item))
  (bind (_itemid_10 _quantity_11) (Utilities|Struct|BreakS_Slots Item))
  (bind (_itemid_11 _quantity_12 _itemtype_9) (Utilities|Struct|BreakS_Slots Item))
  (bind (_itemid_12 _quantity_13) (Utilities|Struct|BreakS_Slots Item))
  (bind (_itemid_13 _quantity_14 _itemtype_10) (Utilities|Struct|BreakS_Slots Item))
  (bind _itemid_14 (Utilities|Struct|BreakS_Slots Item))
  (bind (_itemid_15 _quantity_15 _itemtype_11) (Utilities|Struct|BreakS_Slots Item))
  (bind _rowname (Utilities|Struct|BreakDataTableRowHandle _itemid_14))
  (switch Utilities|FlowControl|Switch|SwitchonE_ItemTypes (.ItemType (Utilities|Struct|BreakS_Slots Item))
    (:NewEnumerator0
      ;[0.6979 0.9003 1] Setup sword inventory
      (for (_array_element _array_index) (.Sword (Utilities|Struct|BreakS_ItemsManager (Variables|Default|GetPlayerInventory)))
        (if (== (.RowName (Utilities|Struct|BreakDataTableRowHandle (.ItemID (Utilities|Struct|BreakS_Slots _array_element)))) (.RowName (Utilities|Struct|BreakDataTableRowHandle (.ItemID (Utilities|Struct|BreakS_Slots Item)))))
          (bind _returnvalue (Utilities|GetDataTableRow "/Game/_Renato/Inventory/Data_Tables/Items/DT_Items.DT_Items" (.RowName (Utilities|Struct|BreakDataTableRowHandle _itemid_12)))
            (:then
              (if (>= (.StackSize (Utilities|Struct|BreakS_Items _returnvalue)) (+ _quantity_13 (.Quantity (Utilities|Struct|BreakS_Slots _array_element))))
                (Utilities|Array|SetArrayElem (.Sword (Utilities|Struct|BreakS_ItemsManager (Variables|Default|GetPlayerInventory))) _array_index (Utilities|Struct|MakeS_Slots _itemid_13 (+ _quantity_13 (.Quantity (Utilities|Struct|BreakS_Slots _array_element))) _itemtype_10))
                (return true)
                (else
                  (return false) ; Should add logic here to fill current slot and then, check if theres an empty slot and add the rest of the stack on it
                ))))))
      (Development|PrintString "We should add to a new slot")
      ;;[0 0.776 1] Search for empty slots
      (bind (_success _array_index_2) (CallFunction|CheckforEmptySlots (.Sword (Utilities|Struct|BreakS_ItemsManager (Variables|Default|GetPlayerInventory))) Item))
      ;;;[0 0.5572 1] Add item to empty slot
      (if _success
        (Utilities|Array|SetArrayElem (.Sword (Utilities|Struct|BreakS_ItemsManager (Variables|Default|GetPlayerInventory))) _array_index_2 Item)
        (return true)
        (else
          (return false))))
    (:NewEnumerator1
      ;[0.5312 0.8453 1] Setup shield inventory
      (for (_array_element_2 _array_index_3) (.Shields (Utilities|Struct|BreakS_ItemsManager (Variables|Default|GetPlayerInventory)))
        (if (== (.RowName (Utilities|Struct|BreakDataTableRowHandle (.ItemID (Utilities|Struct|BreakS_Slots _array_element_2)))) (.RowName (Utilities|Struct|BreakDataTableRowHandle (.ItemID (Utilities|Struct|BreakS_Slots Item)))))
          (bind _returnvalue_2 (Utilities|GetDataTableRow "/Game/_Renato/Inventory/Data_Tables/Items/DT_Items.DT_Items" (.RowName (Utilities|Struct|BreakDataTableRowHandle _itemid_5)))
            (:then
              (if (>= (.StackSize (Utilities|Struct|BreakS_Items _returnvalue_2)) (+ _quantity_6 (.Quantity (Utilities|Struct|BreakS_Slots _array_element_2))))
                (Utilities|Array|SetArrayElem (.Shields (Utilities|Struct|BreakS_ItemsManager (Variables|Default|GetPlayerInventory))) _array_index_3 (Utilities|Struct|MakeS_Slots _itemid_3 (+ _quantity_6 (.Quantity (Utilities|Struct|BreakS_Slots _array_element_2))) _itemtype_3))
                (return true)
                (else
                  (return false) ; Should add logic here to fill current slot and then, check if theres an empty slot and add the rest of the stack on it
                ))))))
      (Development|PrintString "We should add to a new slot")
      ;;[0 0.776 1] Search for empty slots
      (bind (_success_2 _array_index_4) (CallFunction|CheckforEmptySlots (.Shields (Utilities|Struct|BreakS_ItemsManager (Variables|Default|GetPlayerInventory))) Item))
      ;;[0 0.5572 1] Add item to empty slot
      (if _success_2
        (Utilities|Array|SetArrayElem (.Shields (Utilities|Struct|BreakS_ItemsManager (Variables|Default|GetPlayerInventory))) _array_index_4 Item)
        (return true)
        (else
          (return false))))
    (:NewEnumerator2
      ;[0.5932 1 0.9801] Setup Items Inventory
      (for (_array_element_3 _array_index_5) (.Items (Utilities|Struct|BreakS_ItemsManager (Variables|Default|GetPlayerInventory)))
        (LocalVariables|SetCurrentElement _array_element_3)
        (LocalVariables|SetCurrentIndex _array_index_5)
        (if (== (.RowName (Utilities|Struct|BreakDataTableRowHandle (.ItemID (Utilities|Struct|BreakS_Slots _array_element_3)))) (.RowName (Utilities|Struct|BreakDataTableRowHandle (.ItemID (Utilities|Struct|BreakS_Slots Item)))))
          (bind _returnvalue_3 (Utilities|GetDataTableRow "/Game/_Renato/Inventory/Data_Tables/Items/DT_Items.DT_Items" (.RowName (Utilities|Struct|BreakDataTableRowHandle _itemid_10)))
            (:then
              (LocalVariables|SetStackSize (.StackSize (Utilities|Struct|BreakS_Items _returnvalue_3)))
              (if (>= (.StackSize (Utilities|Struct|BreakS_Items _returnvalue_3)) (+ _quantity_11 (.Quantity (Utilities|Struct|BreakS_Slots _array_element_3))))
                (Utilities|Array|SetArrayElem (.Items (Utilities|Struct|BreakS_ItemsManager (Variables|Default|GetPlayerInventory))) _array_index_5 (Utilities|Struct|MakeS_Slots _itemid_11 (+ _quantity_11 (.Quantity (Utilities|Struct|BreakS_Slots _array_element_3))) _itemtype_9))
                (return true)
                (elif (> (.Quantity (Utilities|Struct|BreakS_Slots Item)) (LocalVariables|GetStackSize))
                  ;[0 0.5123 1] Check if we pick an item with more than stack size
                  (if (< (.Quantity (Utilities|Struct|BreakS_Slots (LocalVariables|GetCurrentElement))) (LocalVariables|GetStackSize))
                    ;[0 0.5641 1] Fill slot up
                    (LocalVariables|SetDifference (- (LocalVariables|GetStackSize) (.Quantity (Utilities|Struct|BreakS_Slots (LocalVariables|GetCurrentElement)))))
                    (Utilities|Array|SetArrayElem (.Items (Utilities|Struct|BreakS_ItemsManager (Variables|Default|GetPlayerInventory))) (LocalVariables|GetCurrentIndex) (Utilities|Struct|MakeS_Slots (.ItemID (Utilities|Struct|BreakS_Slots (LocalVariables|GetCurrentElement))) (+ (.Quantity (Utilities|Struct|BreakS_Slots (LocalVariables|GetCurrentElement))) (LocalVariables|GetDifference)) (.ItemType (Utilities|Struct|BreakS_Slots (LocalVariables|GetCurrentElement)))))
                    (LocalVariables|SetRemainder (- (.Quantity (Utilities|Struct|BreakS_Slots Item)) (LocalVariables|GetDifference)))
                    (bind (_success_3 _array_index_6) (CallFunction|CheckforEmptySlots (.Items (Utilities|Struct|BreakS_ItemsManager (Variables|Default|GetPlayerInventory))) Item))
                    (if _success_3
                      ;[0 0.5173 1] If empty slot is found, add remainder to empty slot
                      (Utilities|Array|SetArrayElem (.Items (Utilities|Struct|BreakS_ItemsManager (Variables|Default|GetPlayerInventory))) _array_index_6 (Utilities|Struct|MakeS_Slots _itemid (LocalVariables|GetRemainder) _itemtype))
                      (return true)
                      (else
                        ;[0 0.6288 1] Leave remainder on floor
                        (Game|SpawnActorfromClass "/Game/_Renato/Inventory/Blueprints/Items/BP_Items.BP_Items_C" (Math|Conversions|ToTransform(Vector) (Transformation|GetActorLocation ItemActor)) "Undefined" "MultiplyWithRoot" 0 (Utilities|Struct|MakeS_Slots _itemid_2 (LocalVariables|GetRemainder) _itemtype_2) 0)
                        (return true))))
                  (elif (<= (+ (.Quantity (Utilities|Struct|BreakS_Slots (LocalVariables|GetCurrentElement))) (.Quantity (Utilities|Struct|BreakS_Slots Item))) (LocalVariables|GetStackSize))
                    ;[0 0.5294 1] Add if stack size is not reached on addition
                    (Utilities|Array|SetArrayElem (.Items (Utilities|Struct|BreakS_ItemsManager (Variables|Default|GetPlayerInventory))) (LocalVariables|GetCurrentIndex) (Utilities|Struct|MakeS_Slots _itemid_15 (+ (.Quantity (Utilities|Struct|BreakS_Slots (LocalVariables|GetCurrentElement))) (.Quantity (Utilities|Struct|BreakS_Slots Item))) _itemtype_11))
                    (return true)
                    (else
                      ;[0 0.394 1] Get important info and fill slot
                      (bind _output_get (LocalVariables|SetDifference (- (LocalVariables|GetStackSize) (.Quantity (Utilities|Struct|BreakS_Slots (LocalVariables|GetCurrentElement))))))
                      (LocalVariables|SetRemainder (- (.Quantity (Utilities|Struct|BreakS_Slots Item)) _output_get))
                      (Utilities|Array|SetArrayElem (.Items (Utilities|Struct|BreakS_ItemsManager (Variables|Default|GetPlayerInventory))) (LocalVariables|GetCurrentIndex) (Utilities|Struct|MakeS_Slots (.ItemID (Utilities|Struct|BreakS_Slots (LocalVariables|GetCurrentElement))) (+ (.Quantity (Utilities|Struct|BreakS_Slots (LocalVariables|GetCurrentElement))) (LocalVariables|GetDifference)) (.ItemType (Utilities|Struct|BreakS_Slots (LocalVariables|GetCurrentElement)))))
                      (bind (_success_4 _array_index_7) (CallFunction|CheckforEmptySlots (.Items (Utilities|Struct|BreakS_ItemsManager (Variables|Default|GetPlayerInventory))) Item))
                      (if _success_4
                        ;[0 0.5173 1] If eempty slot is found, add remainder to empty slot
                        (Utilities|Array|SetArrayElem (.Items (Utilities|Struct|BreakS_ItemsManager (Variables|Default|GetPlayerInventory))) _array_index_7 (Utilities|Struct|MakeS_Slots _itemid_8 (LocalVariables|GetRemainder) _itemtype_7))
                        (return true)
                        (else
                          ;[0 0.6288 1] Leave remainder on floor
                          (Game|SpawnActorfromClass "/Game/_Renato/Inventory/Blueprints/Items/BP_Items.BP_Items_C" (Math|Conversions|ToTransform(Vector) (Transformation|GetActorLocation ItemActor)) "Undefined" "MultiplyWithRoot" 0 (Utilities|Struct|MakeS_Slots _itemid_9 (LocalVariables|GetRemainder) _itemtype_8) 0)
                          (return true)))))))))))
      ;;[0 0.776 1] Search for empty slots
      (bind (_success_5 _array_index_8) (CallFunction|CheckforEmptySlots (.Items (Utilities|Struct|BreakS_ItemsManager (Variables|Default|GetPlayerInventory))) Item))
      (if _success_5
        (bind _returnvalue_4 (Utilities|GetDataTableRow "/Game/_Renato/Inventory/Data_Tables/Items/DT_Items.DT_Items" (.RowName (Utilities|Struct|BreakDataTableRowHandle (.ItemID (Utilities|Struct|BreakS_Slots Item)))))
          (:then
            (LocalVariables|SetStackSize (.StackSize (Utilities|Struct|BreakS_Items _returnvalue_4)))
            ;;[0 0.5641 1] Fill slot up
            (if (> _quantity_3 (LocalVariables|GetStackSize))
              (LocalVariables|SetDifference (- _quantity_3 (LocalVariables|GetStackSize)))
              (Utilities|Array|SetArrayElem (.Items (Utilities|Struct|BreakS_ItemsManager (Variables|Default|GetPlayerInventory))) _array_index_8 (Utilities|Struct|MakeS_Slots _itemid_7 (LocalVariables|GetStackSize) _itemtype_6))
              (bind (_success_6 _array_index_9) (CallFunction|CheckforEmptySlots (.Items (Utilities|Struct|BreakS_ItemsManager (Variables|Default|GetPlayerInventory))) Item))
              (if _success_6
                ;[0 0.5173 1] If empty slot is found, add remainder to empty slot
                (Utilities|Array|SetArrayElem (.Items (Utilities|Struct|BreakS_ItemsManager (Variables|Default|GetPlayerInventory))) _array_index_9 (Utilities|Struct|MakeS_Slots _itemid_4 (LocalVariables|GetDifference) _itemtype_4))
                (return true)
                (else
                  ;[0 0.6288 1] Leave remainder on floor
                  (Game|SpawnActorfromClass "/Game/_Renato/Inventory/Blueprints/Items/BP_Items.BP_Items_C" (Math|Conversions|ToTransform(Vector) (Transformation|GetActorLocation ItemActor)) "Undefined" "MultiplyWithRoot" 0 (Utilities|Struct|MakeS_Slots _itemid_6 (LocalVariables|GetDifference) _itemtype_5) 0)
                  (return true)))
              (else
                ;[0 0.5572 1] Add item to empty slot
                (Utilities|Array|SetArrayElem (.Items (Utilities|Struct|BreakS_ItemsManager (Variables|Default|GetPlayerInventory))) _array_index_8 Item)
                (return true)))))))
    (:NewEnumerator3
      ;[0 0.5831 1] Upgrade when picking pack
      (if (== _rowname "WeaponPack")
        (bind _returnvalue_5 (Utilities|GetDataTableRow "/Game/_Renato/Inventory/Data_Tables/Items/DT_Items.DT_Items" _rowname)
          (:then
            (CallFunction|UpgradeInventory (Math|Float|Truncate (.Power (Utilities|Struct|BreakS_Items _returnvalue_5))))))
        (elif (== _rowname "ItemPack")
          (bind _returnvalue_6 (Utilities|GetDataTableRow "/Game/_Renato/Inventory/Data_Tables/Items/DT_Items.DT_Items" (.RowName (Utilities|Struct|BreakDataTableRowHandle (.ItemID (Utilities|Struct|BreakS_Slots Item)))))
            (:then
              (CallFunction|UpgradeInventory 0 0 (Math|Float|Truncate (.Power (Utilities|Struct|BreakS_Items _returnvalue_6))))))
          (else
            (bind _returnvalue_7 (Utilities|GetDataTableRow "/Game/_Renato/Inventory/Data_Tables/Items/DT_Items.DT_Items" (.RowName (Utilities|Struct|BreakDataTableRowHandle (.ItemID (Utilities|Struct|BreakS_Slots Item)))))
              (:then
                (CallFunction|UpgradeInventory 0 (Math|Float|Truncate (.Power (Utilities|Struct|BreakS_Items _returnvalue_7)))))))))
      (return true))))

(fn CheckforEmptySlots
  (params (Array :type Array%20of%20S%20Slots%20Structures) (Item :type S%20Slots%20Structure))
  ;[0 0.776 1] Search for empty slots
  (for (_array_element _array_index) Array
    (Utilities|GetDataTableRow "/Game/_Renato/Inventory/Data_Tables/Items/DT_Items.DT_Items" (.RowName (Utilities|Struct|BreakDataTableRowHandle (.ItemID (Utilities|Struct|BreakS_Slots Item))))
      (:then
        (if (== (.Quantity (Utilities|Struct|BreakS_Slots _array_element)) 0)
          (return true _array_index)
          (else
            (Development|PrintString "Stack size too big, either noob developer or lack of upgrades") ; This could be a result of bad ammo and slot managment so adding this logic to avoid pickup is fine, can expand on it to fill 2 slots or more instead of doing nothing
          )))))
  (return false 0))

(fn UpgradeInventory
  (params (MeleeAmount :type Integer) (OffHandAmount :type Integer) (ItemAmount :type Integer))
  (bind _playerinventory (Variables|Default|GetPlayerInventory))
  (bind (_sword _shields _items) (Utilities|Struct|BreakS_ItemsManager _playerinventory))
  ;[0 0.7223 1] Initialize inventory slot size
  (Utilities|Array|Resize _sword (+ MeleeAmount (Utilities|Array|Length _sword)))
  (Utilities|Array|Resize _shields (+ OffHandAmount (Utilities|Array|Length _shields)))
  (Utilities|Array|Resize _items (+ (Utilities|Array|Length _items) ItemAmount))
  (Default|UpdateItemsinInventoryUI (Variables|Widgets|GetWBP_InventoryWidget) (Variables|Default|GetPlayerInventory)))

(fn SetInventorySize
  (params (MainHandSize :type Integer) (OffHandSize :type Integer) (ItemSize :type Integer))
  (bind _playerinventory (Variables|Default|GetPlayerInventory))
  (bind (_sword _shields _items) (Utilities|Struct|BreakS_ItemsManager _playerinventory))
  ;[0 0.7223 1] Initialize inventory slot size
  (Utilities|Array|Resize _sword MainHandSize)
  (Utilities|Array|Resize _shields OffHandSize)
  (Utilities|Array|Resize _items ItemSize)
  ;[0 0.3769 1] Update Items in inventory in UI
  (Default|UpdateItemsinInventoryUI (Variables|Widgets|GetWBP_InventoryWidget) (Variables|Default|GetPlayerInventory)))