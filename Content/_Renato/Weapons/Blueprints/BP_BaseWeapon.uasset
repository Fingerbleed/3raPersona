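; Base weapon Blueprint providing hitscan firing and inventory-fed reloading, with empty start and stop shooting events.
; FireWeapon traces from the player's follow camera: single shots damage Enemigo actors, while shotgun mode fires five random-spread traces without applying damage.
; Reload refills the magazine through UpdateAmmoInventory, which draws from the largest stack of HandgunAmmo, hardcoded as the ammo type, and refreshes the inventory widget.
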(event Custom|Stop%20shooting)

(event Custom|Start%20Shooting
  (params (Power :type Float%20%28double-precision%29)))

(fn ConstructionScript)

(fn FireWeapon
  (params (WeaponRange :type Float%20%28double-precision%29) (Power :type Float%20%28double-precision%29) (isShotgun :type Boolean))
  (bind _playerref (Variables|Default|GetPlayerRef))
  (bind _spread (Variables|Default|GetSpread))
  (bind _spread_2 (Variables|Default|GetSpread))
  (bind _spread_3 (Variables|Default|GetSpread))
  (bind _playerref_2 (Variables|Default|GetPlayerRef))
  (bind _followcamera (Variables|/Game/ThirdPerson/Blueprints/BP_ThirdPersonCharacter.BP_ThirdPersonCharacter_C|GetFollowCamera _playerref))
  (bind _followcamera_2 (Variables|/Game/ThirdPerson/Blueprints/BP_ThirdPersonCharacter.BP_ThirdPersonCharacter_C|GetFollowCamera _playerref_2))
  (bind _returnvalue (Transformation|GetWorldLocation _followcamera_2))
  (bind _returnvalue_2 (Transformation|GetWorldLocation _followcamera))
  (if (> (Variables|Default|GetCurrentAmmo) 0)
    (if isShotgun
      (Variables|Default|SetPlayAnimation? true)
      (for _index (range 1 5)
        (bind _outhit (Collision|LineTraceByChannel _returnvalue (+ _returnvalue (* (Math|Vector|GetForwardVector _followcamera_2) WeaponRange) (Math|Vector|MakeVector (Math|Random|RandomFloatinRange (* _spread_2 -1.0) _spread_2) (Math|Random|RandomFloatinRange (* _spread_3 -1.0) _spread_3) (Math|Random|RandomFloatinRange (* _spread -1.0) _spread))) "TraceTypeQuery2" false (Utilities|Array|MakeArray (Game|GetPlayerCharacter 0)) "ForDuration")))
      (Math|Integer|DecrementInt (Variables|Default|GetCurrentAmmo))
      (else
        (Variables|Default|SetPlayAnimation? true)
        (bind _outhit_2 (Collision|LineTraceByChannel _returnvalue_2 (+ (* (Math|Vector|GetForwardVector _followcamera) WeaponRange) _returnvalue_2) "TraceTypeQuery1" false (Utilities|Array|MakeArray (Game|GetPlayerCharacter 0)) "ForDuration"))
        (Math|Integer|DecrementInt (Variables|Default|GetCurrentAmmo)
          (:%20%20
            (bind _asenemigo (Utilities|Casting|CastToEnemigo (.HitActor (Collision|BreakHitResult _outhit_2))))
            (Game|Damage|ApplyDamage _asenemigo Power 0 0)))))
    (else
      (Variables|Default|SetPlayAnimation? false))))

(fn Reload
  (if (> (Variables|Default|GetAmmoInInventory) 0)
    (bind _output_get (LocalVariables|SetAmmoDifference (- (Variables|Default|GetMagSize) (Variables|Default|GetCurrentAmmo))))
    (bind (_ammoleftover _fullmag) (CallFunction|UpdateAmmoInventory _output_get))
    (if _fullmag
      (Variables|Default|SetCurrentAmmo _ammoleftover)
      (else
        (Variables|Default|SetCurrentAmmo (+ _ammoleftover (Variables|Default|GetCurrentAmmo)))))
    (Development|PrintString "Reloading")))

(fn UpdateAmmoInventory
  (params (AmmoUsed :type Integer))
  (bind _playerref (Variables|Default|GetPlayerRef))
  (bind _playerref_2 (Variables|Default|GetPlayerRef))
  (bind _bpc_inventorymanager (Variables|/Game/ThirdPerson/Blueprints/BP_ThirdPersonCharacter.BP_ThirdPersonCharacter_C|GetBPC_InventoryManager _playerref))
  (bind _bpc_inventorymanager_2 (Variables|/Game/ThirdPerson/Blueprints/BP_ThirdPersonCharacter.BP_ThirdPersonCharacter_C|GetBPC_InventoryManager _playerref_2))
  (for (_array_element _array_index) (.Items (Utilities|Struct|BreakS_ItemsManager (Variables|/Game/_Renato/Inventory/Components/BPC_InventoryManager.BPC_InventoryManager_C|GetPlayerInventory (Variables|/Game/ThirdPerson/Blueprints/BP_ThirdPersonCharacter.BP_ThirdPersonCharacter_C|GetBPC_InventoryManager (Variables|Default|GetPlayerRef)))))
    (if (== (.RowName (Utilities|Struct|BreakDataTableRowHandle (.ItemID (Utilities|Struct|BreakS_Slots _array_element)))) "HandgunAmmo")
      (if (> (.Quantity (Utilities|Struct|BreakS_Slots _array_element)) (LocalVariables|GetBiggestStack))
        (LocalVariables|SetStackIndex _array_index)
        (LocalVariables|SetBiggestStack (.Quantity (Utilities|Struct|BreakS_Slots _array_element))))))
  (if (>= AmmoUsed (LocalVariables|GetBiggestStack))
    ;[0 0.5727 1] Empty up slot since ammo in inventory + mag size is less than a full mag
    (Utilities|Array|SetArrayElem (.Items (Utilities|Struct|BreakS_ItemsManager (Variables|/Game/_Renato/Inventory/Components/BPC_InventoryManager.BPC_InventoryManager_C|GetPlayerInventory (Variables|/Game/ThirdPerson/Blueprints/BP_ThirdPersonCharacter.BP_ThirdPersonCharacter_C|GetBPC_InventoryManager (Variables|Default|GetPlayerRef))))) (LocalVariables|GetStackIndex) (Utilities|Struct|MakeS_Slots (Utilities|Struct|MakeDataTableRowHandle "/Game/_Renato/Inventory/Data_Tables/Items/DT_Items.DT_Items" "HandgunAmmo") 0 "NewEnumerator2"))
    (Default|UpdateItemsinInventoryUI (Variables|/Game/_Renato/Inventory/Components/BPC_InventoryManager.BPC_InventoryManager_C|GetWBP_InventoryWidget _bpc_inventorymanager) (Variables|/Game/_Renato/Inventory/Components/BPC_InventoryManager.BPC_InventoryManager_C|GetPlayerInventory _bpc_inventorymanager))
    (return (LocalVariables|GetBiggestStack) false)
    (else
      ;[0 0.4576 1] Set slot to ammo remainder
      (Utilities|Array|SetArrayElem (.Items (Utilities|Struct|BreakS_ItemsManager (Variables|/Game/_Renato/Inventory/Components/BPC_InventoryManager.BPC_InventoryManager_C|GetPlayerInventory (Variables|/Game/ThirdPerson/Blueprints/BP_ThirdPersonCharacter.BP_ThirdPersonCharacter_C|GetBPC_InventoryManager (Variables|Default|GetPlayerRef))))) (LocalVariables|GetStackIndex) (Utilities|Struct|MakeS_Slots (Utilities|Struct|MakeDataTableRowHandle "/Game/_Renato/Inventory/Data_Tables/Items/DT_Items.DT_Items" "HandgunAmmo") (- (LocalVariables|GetBiggestStack) AmmoUsed) "NewEnumerator2"))
      (Default|UpdateItemsinInventoryUI (Variables|/Game/_Renato/Inventory/Components/BPC_InventoryManager.BPC_InventoryManager_C|GetWBP_InventoryWidget _bpc_inventorymanager_2) (Variables|/Game/_Renato/Inventory/Components/BPC_InventoryManager.BPC_InventoryManager_C|GetPlayerInventory _bpc_inventorymanager_2))
      (return (Variables|Default|GetMagSize) true))))